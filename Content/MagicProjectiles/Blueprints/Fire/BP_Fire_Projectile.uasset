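; Fire projectile actor that acts as a firebomb, spawning a muzzle effect at launch and exploding after a short fuse on overlap or a lifetime timeout.
; On overlap it calls an actor attach, stops its movement and waits before detonating.
; Detonation spawns an explosion emitter, sends the actors overlapping Sphere1 to the owner as Gameplay Ability System target data in a Firebomb explosion event, then destroys the projectile.
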(event `self.ReceiveBeginPlay`
  (`NiagaraFunctionLibrary.SpawnSystemAtLocation` "/Game/MagicProjectiles/Niagara/Fire/NS_Fire_Muzzle.NS_Fire_Muzzle" (`self.K2_GetActorLocation`))
  (`KismetSystemLibrary.Delay` 5.0)
  (`GameplayStatics.SpawnEmitterAtLocation` "/Game/FXVarietyPack/Particles/P_ky_explosion.P_ky_explosion" (`self.K2_GetActorLocation`) (struct) (2.0 2.0 2.0))
  (`AbilitySystemBlueprintLibrary.SendGameplayEventToActor` (`self.GetOwner`) (struct :`TagName` "Ability.Firebomb.Explosion") (make `GameplayEventData` (struct) null null null null (struct) (struct) (struct) 0.0 (`AbilitySystemBlueprintLibrary.AbilityTargetDataFromActorArray` (`PrimitiveComponent.GetOverlappingActors` (`self.Sphere1`) "/Script/Engine.Actor") true)))
  (`self.K2_DestroyActor`))

(event `self.Sphere.OnComponentBeginOverlap`
  (params (OverlappedComponent :type "PrimitiveComponent Object Reference") (OtherActor :type "Actor Object Reference") (OtherComp :type "PrimitiveComponent Object Reference") (OtherBodyIndex :type Integer) (bFromSweep :type Boolean) (SweepResult :type "HitResult Structure (by ref)"))
  (if (!= OtherActor self)
    (`self.K2_AttachToActor` null "None" "KeepWorld" "KeepWorld" "KeepWorld"))
  (`MovementComponent.StopMovementImmediately` (`self.ProjectileMovement`))
  (`KismetSystemLibrary.Delay` 1.5)
  (`PrimitiveComponent.SetCollisionResponseToAllChannels` (`self.Sphere1`) (`self.New Response`))
  (`GameplayStatics.SpawnEmitterAtLocation` "/Game/FXVarietyPack/Particles/P_ky_explosion.P_ky_explosion" (`self.K2_GetActorLocation`) (struct) (2.0 2.0 2.0))
  (`AbilitySystemBlueprintLibrary.SendGameplayEventToActor` (`self.GetOwner`) (struct :`TagName` "Ability.Firebomb.Explosion") (make `GameplayEventData` (struct) null null null null (struct) (struct) (struct) 0.0 (`AbilitySystemBlueprintLibrary.AbilityTargetDataFromActorArray` (`PrimitiveComponent.GetOverlappingActors` (`self.Sphere1`) "/Script/Engine.Actor") true)))
  (`self.K2_DestroyActor`))

(fn `UserConstructionScript`
  (`parent.UserConstructionScript`))