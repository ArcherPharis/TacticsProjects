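; BP_WaterSource is a crafting pickup that is triggered when an actor carrying the fire tag overlaps its sphere.
; On overlap it gets player 0's BP_PlayerCharacter, not the overlapping actor, and applies the EffectUponPickup gameplay effect through its Ability System Component.
; It then spawns a hit particle at its own location and calls PickupItem for that player.
; The Interactwith event is left empty.
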(event `self.ReceiveBeginPlay`)

(event `InteractInterface.InteractWith`
  (params (player :type "PlayerCharacter Object Reference")))

(event `self.Sphere.OnComponentBeginOverlap`
  (params (OverlappedComponent :type "PrimitiveComponent Object Reference") (OtherActor :type "Actor Object Reference") (OtherComp :type "PrimitiveComponent Object Reference") (OtherBodyIndex :type Integer) (bFromSweep :type Boolean) (SweepResult :type "HitResult Structure (by ref)"))
  (if (`self.ActorHasTag` OtherActor (`self.FireTag`))
    (bind _asbp_player_character (cast `/Game/Blueprints/Player/BP_PlayerCharacter` (`GameplayStatics.GetPlayerCharacter` 0)))
    (`AbilitySystemComponent.BP_ApplyGameplayEffectToSelf` :`self` (`AbilitySystemBlueprintLibrary.GetAbilitySystemComponent` _asbp_player_character) :`GameplayEffectClass` (`self.EffectUponPickup`))
    (`GameplayStatics.SpawnEmitterAtLocation` "/Game/FXVarietyPack/Particles/P_ky_hit1.P_ky_hit1" (`self.K2_GetActorLocation`))
    (`self.PickupItem` self _asbp_player_character)))

(fn `UserConstructionScript`
  (`parent.UserConstructionScript`))