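; BP_BaseItem is a base item actor that a player can pick up into their inventory.
; PickupItem plays a pickup sound and adds one of the item's own class to the passed player's inventory component.
; It then refreshes the inventory in WBP_InGameUI through player 0's BP_PlayerController and destroys itself, which is skipped if either cast fails.
; The event graph and construction script are empty, so PickupItem must be called externally.
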(fn `PickupItem`
  (params (Player :type "PlayerCharacter Object Reference"))
  (`GameplayStatics.PlaySound2D` "/Engine/VREditor/Sounds/UI/Object_PickUp.Object_PickUp" 1.0 1.0 0.0 null null)
  (`InventoryComponent.AddToInventory` (`PlayerCharacter.GetInventoryComponent` Player) (`GameplayStatics.GetObjectClass` self) 1)
  (bind _asbp_player_controller (cast `/Game/Blueprints/Controllers/BP_PlayerController` (`GameplayStatics.GetPlayerController` 0)))
  (bind _aswbp_in_game_ui (cast `/Game/Blueprints/Widgets/WBP_InGameUI` (`LVPlayerController.GetUI` _asbp_player_controller)))
  (`/Game/Blueprints/Widgets/WBP_InGameUI.RefreshInventory` _aswbp_in_game_ui)
  (`self.K2_DestroyActor`))

(fn `UserConstructionScript`)